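; Interactable weapon crate that shows a "To Open" prompt and yields a weapon, ammo and supplies.
; Interact sends the player three spawn locations in front of the crate and a self reference through OpenCrateMessage, then removes the prompt and box.
; SpawnSupplies tilts the lid mesh and spawns the given weapon and ammo classes at matching offsets.
; The local random ammo and extra-supply selection is disconnected and never runs.
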(event `self.ReceiveBeginPlay`
  (bind _asinteract_ui (cast `/Game/MyPlayer/Widget/Interact_UI` (`WidgetComponent.GetUserWidgetObject` (`self.Widget`))))
  (set `/Game/MyPlayer/Widget/Interact_UI.Interact Text` "To Open" _asinteract_ui))

(event `/Game/MyPlayer/OtherBlueprints/Player_BPI.Show Interaction Widget`
  (params (Visibility :type Boolean))
  (`/Engine/EditorBlueprintResources/StandardMacros.IsValid` (`self.Widget`)
    (:`Is Valid`
      (`SceneComponent.SetVisibility` (`self.Widget`) Visibility false))))

(event `Spawn Supplies`
  (params (`Weapon Class` :type "Actor Class Reference") (`Ammo Class` :type "Actor Class Reference"))
  (bind (_returnvalue_roll _returnvalue_pitch _returnvalue_yaw) (`KismetMathLibrary.BreakRotator` (`self.K2_GetActorRotation`)))
  (`SceneComponent.K2_SetRelativeRotation` (`self.WeaponCrate_defaultMaterial_004`) (struct :`Roll` -80.0) false false)
  (`KismetSystemLibrary.PrintString` "Hello")
  (`|SpawnActorFromClass` `Weapon Class` (`KismetMathLibrary.MakeTransform` (+ (+ (+ (`self.K2_GetActorLocation`) (* (`self.GetActorForwardVector`) 100.0)) (0.0 0.0 6.0)) (* (`self.GetActorRightVector`) -60.0)) (`KismetMathLibrary.MakeRotator` _returnvalue_roll 90.0 _returnvalue_yaw)) "Undefined" "MultiplyWithRoot" null null)
  (`|SpawnActorFromClass` `Ammo Class` (`KismetMathLibrary.MakeTransform` (+ (+ (`self.K2_GetActorLocation`) (* (`self.GetActorForwardVector`) 100.0)) (* (`self.GetActorRightVector`) 20.0))) "Undefined" "MultiplyWithRoot" null null))

(event `/Game/MyPlayer/OtherBlueprints/Player_BPI.Interact`
  (params (Player :type "Pawn Object Reference"))
  (message `/Game/MyPlayer/OtherBlueprints/Player_BPI.Open Crate` Player (+ (+ (+ (`self.K2_GetActorLocation`) (* (`self.GetActorForwardVector`) 100.0)) (0.0 0.0 6.0)) (* (`self.GetActorRightVector`) -60.0)) (+ (+ (`self.K2_GetActorLocation`) (* (`self.GetActorForwardVector`) 100.0)) (* (`self.GetActorRightVector`) 20.0)) (+ (+ (`self.K2_GetActorLocation`) (* (`self.GetActorForwardVector`) 100.0)) (* (`self.GetActorRightVector`) 60.0)) self)
  (`ActorComponent.K2_DestroyComponent` (`self.Widget`))
  (`ActorComponent.K2_DestroyComponent` (`self.Box`)))

(fn `Hand Sway`
  (returns (SideMov :type "Float (double-precision)") (`Mouse X` :type "Float (double-precision)") (`Mouse Y` :type "Float (double-precision)"))
  (return 0.0 0.0 0.0))

(fn `Hand Sway 2`
  (returns (`Front Mov` :type "Float (double-precision)"))
  (return 0.0))

(fn `UserConstructionScript`)