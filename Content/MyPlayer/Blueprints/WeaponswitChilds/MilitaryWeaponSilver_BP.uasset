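; MilitaryWeaponSilver_BP is a pickup weapon Blueprint for a silver Scar-L rifle, built on a parent weapon class.
; On BeginPlay it writes the weapon name and preview image into its PickupWeapon_UI widget, and toggles two widget components' visibility as the interaction prompt.
; Interacting passes its weapon enum and itself to the player, then disables the Box collision.
; Both hand sway functions return only zeros.
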(event `self.ReceiveBeginPlay`
  (`parent.ReceiveBeginPlay`)
  (bind _aspickup_weapon_ui (cast `/Game/MyPlayer/Widget/PickupWeapon_UI` (`WidgetComponent.GetUserWidgetObject` (`self.Widget1`))))
  (set `/Game/MyPlayer/Widget/PickupWeapon_UI.Name` "Scar - L" _aspickup_weapon_ui)
  (set `/Game/MyPlayer/Widget/PickupWeapon_UI.Image` "/Game/MyPlayer/Images/Weaponsicons/Pi7_Sivler-removebg-preview.Pi7_Sivler-removebg-preview" _aspickup_weapon_ui))

(event `self.Show Interaction Widget`
  (params (Visibility :type Boolean))
  (`SceneComponent.SetVisibility` (`self.Widget`) Visibility false)
  (`SceneComponent.SetVisibility` (`self.Widget1`) Visibility false))

(event `self.Interact`
  (params (Player :type "Pawn Object Reference"))
  (message `/Game/MyPlayer/OtherBlueprints/Player_BPI.Pickup Weapon` Player "NewEnumerator8" self)
  (`self.CustomEvent`))

(event `CustomEvent`
  (`PrimitiveComponent.SetCollisionEnabled` (`self.Box`) "NoCollision"))

(fn `Hand Sway`
  (returns (SideMov :type "Float (double-precision)") (`Mouse X` :type "Float (double-precision)") (`Mouse Y` :type "Float (double-precision)"))
  (return 0.0 0.0 0.0))

(fn `Hand Sway 2`
  (returns (`Front Mov` :type "Float (double-precision)"))
  (return 0.0))

(fn `UserConstructionScript`
  (`parent.UserConstructionScript`))