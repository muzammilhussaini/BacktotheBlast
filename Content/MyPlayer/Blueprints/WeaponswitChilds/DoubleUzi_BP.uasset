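; DoubleUzi_BP is a dual Uzi weapon pickup, a child weapon Blueprint that responds to interaction.
; Showing the prompt toggles its widget and adds or removes a pickup UI, which is labelled "Assault Rifle" with the rifle icon.
; Interact notifies the player of the pickup, disables box collision and snaps WeaponMesh1 to the player's LeftWeaponSocket.
; Both hand sway functions are stubs returning zero.
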(event `self.Show Interaction Widget`
  (params (Visibility :type Boolean))
  (`SceneComponent.SetVisibility` (`self.Widget`) Visibility false)
  (if Visibility
    (bind _returnvalue (`|CreateWidget` "/Game/MyPlayer/Widget/PickupWeapon_UI.PickupWeapon_UI_C" null 1 "Assault Rifle" "/Game/MyPlayer/Images/Weaponsicons/RifleIcon.RifleIcon"))
    (`UserWidget.AddToViewport` _returnvalue 0)
    (else
      (`/Engine/EditorBlueprintResources/StandardMacros.IsValid` _returnvalue
        (:`Is Valid`
          (`Widget.RemoveFromParent` _returnvalue))))))

(event `self.Interact`
  (params (Player :type "Pawn Object Reference"))
  (message `/Game/MyPlayer/OtherBlueprints/Player_BPI.Pickup Weapon` Player "NewEnumerator10" self)
  (`PrimitiveComponent.SetCollisionEnabled` (`self.Box`) "NoCollision")
  (bind _asplayer_bp (cast `/Game/MyPlayer/Player_BP` Player))
  (`SceneComponent.K2_AttachToComponent` (`self.Weapon Mesh1`) (`Character.Mesh` _asplayer_bp) "LeftWeaponSocket" "SnapToTarget" "SnapToTarget" "SnapToTarget" true))

(fn `Hand Sway`
  (returns (SideMov :type "Float (double-precision)") (`Mouse X` :type "Float (double-precision)") (`Mouse Y` :type "Float (double-precision)"))
  (return 0.0 0.0 0.0))

(fn `Hand Sway 2`
  (returns (`Front Mov` :type "Float (double-precision)"))
  (return 0.0))

(fn `UserConstructionScript`
  (`parent.UserConstructionScript`))