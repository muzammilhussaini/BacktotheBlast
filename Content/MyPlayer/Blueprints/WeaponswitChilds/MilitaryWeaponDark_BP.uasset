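; MilitaryWeaponDark_BP is a child weapon Blueprint for a rifle pickup labeled "m416" in its pickup widget.
; On BeginPlay it sets that widget's name and rifle icon, and an interaction event toggles the visibility of both widget components.
; Interacting sends the player a pickup message with the weapon type and itself, then disables the Box collision.
; The hand sway functions return only zeros.
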(event `self.ReceiveBeginPlay`
  (`parent.ReceiveBeginPlay`)
  (bind _aspickup_weapon_ui (cast `/Game/MyPlayer/Widget/PickupWeapon_UI` (`WidgetComponent.GetUserWidgetObject` (`self.Widget1`))))
  (set `/Game/MyPlayer/Widget/PickupWeapon_UI.Name` "m416" _aspickup_weapon_ui)
  (set `/Game/MyPlayer/Widget/PickupWeapon_UI.Image` "/Game/MyPlayer/Images/Weaponsicons/RifleIcon.RifleIcon" _aspickup_weapon_ui))

(event `self.Show Interaction Widget`
  (params (Visibility :type Boolean))
  (`SceneComponent.SetVisibility` (`self.Widget`) Visibility false)
  (`SceneComponent.SetVisibility` (`self.Widget1`) Visibility false))

(event `self.Interact`
  (params (Player :type "Pawn Object Reference"))
  (message `/Game/MyPlayer/OtherBlueprints/Player_BPI.Pickup Weapon` Player "NewEnumerator7" self)
  (`self.CustomEvent`))

(event `CustomEvent`
  (`PrimitiveComponent.SetCollisionEnabled` (`self.Box`) "NoCollision"))

(fn `Hand Sway`
  (returns (SideMov :type "Float (double-precision)") (`Mouse X` :type "Float (double-precision)") (`Mouse Y` :type "Float (double-precision)"))
  (return 0.0 0.0 0.0))

(fn `Hand Sway 2`
  (returns (`Front Mov` :type "Float (double-precision)"))
  (return 0.0))

(fn `UserConstructionScript`
  (`parent.UserConstructionScript`))