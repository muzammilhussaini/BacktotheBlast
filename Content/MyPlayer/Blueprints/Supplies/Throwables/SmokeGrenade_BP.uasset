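; Throwable smoke grenade that a player lobs to produce a timed smoke cloud.
; Throw turns on physics and collision on the mesh, then applies a forward, upward and slightly rightward impulse from the target's orientation.
; A BeginPlay timer, independent of the throw, spawns an attached smoke particle system after a fuse delay, later deactivates it and destroys the actor.
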(event `self.ReceiveBeginPlay`
  (`KismetSystemLibrary.Delay` 5.0)
  (bind _returnvalue (`NiagaraFunctionLibrary.SpawnSystemAttached` "/Game/M5VFXVOL2/Niagara/Reference/Smoke/5_6_Nsmoke6_pt2.5_6_Nsmoke6_pt2" (`self.StaticMeshComponent`) "None" (- (`SceneComponent.K2_GetComponentLocation` (`self.StaticMeshComponent`)) (0.0 0.0 30.0)) (struct) "KeepWorldPosition"))
  (`KismetSystemLibrary.Delay` 15.0)
  (`ActorComponent.Deactivate` _returnvalue)
  (`KismetSystemLibrary.Delay` 2.5)
  (`self.K2_DestroyActor`))

(event `Throw`
  (params (Target :type "CameraComponent Object Reference"))
  (bind _staticmeshcomponent (`self.StaticMeshComponent`))
  (`PrimitiveComponent.SetSimulatePhysics` _staticmeshcomponent true)
  (`PrimitiveComponent.SetCollisionEnabled` (`self.StaticMeshComponent`) "QueryAndPhysics")
  (`PrimitiveComponent.AddImpulse` _staticmeshcomponent (+ (+ (* (`SceneComponent.GetForwardVector` Target) 3000.0) (* (`SceneComponent.GetUpVector` Target) 500.0)) (* (`SceneComponent.GetRightVector` Target) 50.0)) "None" false))

(fn `Hand Sway`
  (returns (SideMov :type "Float (double-precision)") (`Mouse X` :type "Float (double-precision)") (`Mouse Y` :type "Float (double-precision)"))
  (return 0.0 0.0 0.0))

(fn `Hand Sway 2`
  (returns (`Front Mov` :type "Float (double-precision)"))
  (return 0.0))

(fn `UserConstructionScript`)