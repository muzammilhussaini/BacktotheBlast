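; Throwable grenade actor that explodes on a two-second fuse started at BeginPlay and then destroys itself.
; Throw enables physics on the mesh and launches it with an impulse along the target's forward, up and right vectors.
; The explosion spawns effects and sound, then runs a debug-drawn sphere trace to send random damage through each hit Player_BP's ApplyDamageOnServer.
; Hand sway functions are empty stubs and ProjectileMovement is unused.
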(event `self.ReceiveBeginPlay`
  (bind _returnvalue (`SceneComponent.K2_GetComponentLocation` (`self.StaticMeshComponent`)))
  (`KismetSystemLibrary.Delay` 2.0)
  (`GameplayStatics.SpawnEmitterAtLocation` "/Game/MilitaryWeapDark/FX/P_Grenade_Explosion_01.P_Grenade_Explosion_01" (`SceneComponent.K2_GetComponentLocation` (`self.StaticMeshComponent`)))
  (`GameplayStatics.PlaySoundAtLocation` "/Game/MyPlayer/Sounds/Sounds/grenade-explosion-14-190266.grenade-explosion-14-190266" (`self.K2_GetActorLocation`) (struct) 1.0 1.0 0.0 "/Game/MyPlayer/Sounds/WeaponSouneds_Attenuation.WeaponSouneds_Attenuation" null null null)
  (bind (_outhits _returnvalue_2) (`KismetSystemLibrary.SphereTraceMultiForObjects` :`Start` _returnvalue :`End` _returnvalue :`Radius` 400.0 :`ObjectTypes` (`|MakeArray` "ObjectTypeQuery8" :!type "EObjectTypeQuery Enum") :`DrawDebugType` "ForDuration"))
  (if _returnvalue_2
    (for _array_element _outhits
      (bind (_bblockinghit _binitialoverlap _time _distance _location _impactpoint _normal _impactnormal _physmat _hitactor) (`GameplayStatics.BreakHitResult` _array_element))
      (bind _asplayer_bp (cast `/Game/MyPlayer/Player_BP` _hitactor))
      (`/Game/MyPlayer/Player_BP.Apply Damage On Server` _asplayer_bp (`KismetMathLibrary.RandomFloatInRange` 60.0 80.0) _hitactor)))
  (`self.K2_DestroyActor`))

(event `Throw`
  (params (Target :type "CameraComponent Object Reference"))
  (bind _staticmeshcomponent (`self.StaticMeshComponent`))
  (`PrimitiveComponent.SetSimulatePhysics` _staticmeshcomponent true)
  (`PrimitiveComponent.SetCollisionEnabled` (`self.StaticMeshComponent`) "QueryAndPhysics")
  (`PrimitiveComponent.AddImpulse` _staticmeshcomponent (+ (+ (* (`SceneComponent.GetForwardVector` Target) 3000.0) (* (`SceneComponent.GetUpVector` Target) 500.0)) (* (`SceneComponent.GetRightVector` Target) 50.0)) "None" false))

(fn `Hand Sway`
  (returns (SideMov :type "Float (double-precision)") (`Mouse X` :type "Float (double-precision)") (`Mouse Y` :type "Float (double-precision)"))
  (return 0.0 0.0 0.0))

(fn `Hand Sway 2`
  (returns (`Front Mov` :type "Float (double-precision)"))
  (return 0.0))

(fn `UserConstructionScript`)