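; Grenade launcher projectile that explodes shortly after landing and damages nearby players.
; From BeginPlay it repeats a short downward line trace until it finds WorldStatic geometry beneath the mesh, then waits out a fuse.
; It spawns explosion effects and sound, then sphere traces around itself with debug drawing left on.
; Each Player_BP hit takes random damage through ApplyDamageOnServer, without distance falloff, and the projectile destroys itself.
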(event `self.ReceiveBeginPlay`
  (bind _returnvalue (`SceneComponent.K2_GetComponentLocation` (`self.GrenadeLauncherB_Ammo`)))
  (bind _returnvalue_2 (`SceneComponent.K2_GetComponentLocation` (`self.GrenadeLauncherB_Ammo`)))
  (bind (_outhit _returnvalue_3) (`KismetSystemLibrary.LineTraceSingleForObjects` _returnvalue (- _returnvalue (0.0 0.0 20.0)) (`|MakeArray` "ObjectTypeQuery1" :!type "EObjectTypeQuery Enum") :!label _label))
  (if _returnvalue_3
    (`KismetSystemLibrary.Delay` 2.0)
    (`GameplayStatics.SpawnEmitterAtLocation` "/Game/Realistic_Starter_VFX_Pack_Vol2/Particles/Explosion/P_Explosion_Big_A.P_Explosion_Big_A" (`SceneComponent.K2_GetComponentLocation` (`self.GrenadeLauncherB_Ammo`)) (struct) (1.7 1.7 1.7))
    (`GameplayStatics.PlaySoundAtLocation` "/Game/MyPlayer/Sounds/Sounds/grenade-explosion-14-190266.grenade-explosion-14-190266" (`self.K2_GetActorLocation`) (struct) 1.0 1.0 0.0 "/Game/MyPlayer/Sounds/WeaponSouneds_Attenuation.WeaponSouneds_Attenuation" null null null)
    (bind (_outhits _returnvalue_4) (`KismetSystemLibrary.SphereTraceMultiForObjects` :`Start` _returnvalue_2 :`End` _returnvalue_2 :`Radius` 400.0 :`ObjectTypes` (`|MakeArray` "ObjectTypeQuery8" :!type "EObjectTypeQuery Enum") :`DrawDebugType` "ForDuration"))
    (if _returnvalue_4
      (for _array_element _outhits
        (bind (_bblockinghit _binitialoverlap _time _distance _location _impactpoint _normal _impactnormal _physmat _hitactor) (`GameplayStatics.BreakHitResult` _array_element))
        (bind _asplayer_bp (cast `/Game/MyPlayer/Player_BP` _hitactor))
        (`/Game/MyPlayer/Player_BP.Apply Damage On Server` _asplayer_bp (`KismetMathLibrary.RandomFloatInRange` 60.0 80.0) _hitactor)))
    (`self.K2_DestroyActor`)
    (else
      (`KismetSystemLibrary.Delay` 0.05)
      (goto _label))))

(fn `UserConstructionScript`)