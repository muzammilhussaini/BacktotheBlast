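; Throwable stun grenade that sends a stun message to nearby actors, then destroys itself.
; Throw enables physics and collision on the mesh and launches it with an impulse built from the target's forward, up and slight right vectors.
; A five-second fuse starts at BeginPlay, independent of Throw, then a multi-sphere object trace finds the actors to message.
; Hand sway functions are zero-returning stubs.
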(event `self.ReceiveBeginPlay`
  (bind _returnvalue (`SceneComponent.K2_GetComponentLocation` (`self.StaticMeshComponent`)))
  (`KismetSystemLibrary.Delay` 5.0)
  (bind (_outhits _returnvalue_2) (`KismetSystemLibrary.SphereTraceMultiForObjects` _returnvalue _returnvalue 500.0 (`|MakeArray` "ObjectTypeQuery8" :!type "EObjectTypeQuery Enum")))
  (if _returnvalue_2
    (for _array_element _outhits
      (message `/Game/MyPlayer/OtherBlueprints/Player_BPI.Apply Stun Grenade` (`.HitActor` (`GameplayStatics.BreakHitResult` _array_element)))))
  (`self.K2_DestroyActor`))

(event `Throw`
  (params (Target :type "CameraComponent Object Reference"))
  (bind _staticmeshcomponent (`self.StaticMeshComponent`))
  (`PrimitiveComponent.SetSimulatePhysics` _staticmeshcomponent true)
  (`PrimitiveComponent.SetCollisionEnabled` (`self.StaticMeshComponent`) "QueryAndPhysics")
  (`PrimitiveComponent.AddImpulse` _staticmeshcomponent (+ (+ (* (`SceneComponent.GetForwardVector` Target) 3000.0) (* (`SceneComponent.GetUpVector` Target) 500.0)) (* (`SceneComponent.GetRightVector` Target) 50.0)) "None" false))

(fn `Hand Sway`
  (returns (SideMov :type "Float (double-precision)") (`Mouse X` :type "Float (double-precision)") (`Mouse Y` :type "Float (double-precision)"))
  (return 0.0 0.0 0.0))

(fn `Hand Sway 2`
  (returns (`Front Mov` :type "Float (double-precision)"))
  (return 0.0))

(fn `UserConstructionScript`)