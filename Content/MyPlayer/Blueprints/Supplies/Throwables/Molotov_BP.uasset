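; Throwable Molotov that shatters on the ground and leaves a temporary fire that damages players.
; Throw enables physics on the mesh and launches it with an impulse along the target's vectors.
; Tick traces briefly downward for static world, then swaps the mesh for break and fire effects with sounds.
; A looping timer sphere-traces around the fire, sending small random damage through Player_BP's server call until the fire expires and the actor is destroyed.
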(event `CustomEvent`
  (bind _returnvalue (`SceneComponent.K2_GetComponentLocation` (stale `self.ReceiveTick` _returnvalue_3)))
  (bind (_outhits _returnvalue_2) (`KismetSystemLibrary.SphereTraceMultiForObjects` :`Start` _returnvalue :`End` _returnvalue :`Radius` 240.0 :`ObjectTypes` (`|MakeArray` "ObjectTypeQuery8" :!type "EObjectTypeQuery Enum") :`DrawDebugType` "ForOneFrame"))
  (if _returnvalue_2
    (for _array_element _outhits
      (bind _asplayer_bp (cast `/Game/MyPlayer/Player_BP` (`.HitActor` (`GameplayStatics.BreakHitResult` _array_element))))
      (`/Game/MyPlayer/Player_BP.Apply Damage On Server` _asplayer_bp (`KismetMathLibrary.RandomFloatInRange` 1.0 2.0) _asplayer_bp))))

(event `self.ReceiveTick`
  (params (DeltaSeconds :type "Float (single-precision)"))
  (bind _returnvalue (`SceneComponent.K2_GetComponentLocation` (`self.StaticMeshComponent`)))
  (if (not (`self.Is Broken?`))
    (bind (_outhit _returnvalue_2) (`KismetSystemLibrary.LineTraceSingleForObjects` _returnvalue (- _returnvalue (0.0 0.0 20.0)) (`|MakeArray` "ObjectTypeQuery1" :!type "EObjectTypeQuery Enum")))
    (if _returnvalue_2
      (`GameplayStatics.PlaySoundAtLocation` "/Game/MyPlayer/Sounds/Sounds/object-break-glass-small-02.object-break-glass-small-02" (`self.K2_GetActorLocation`) (struct) 1.0 1.0 0.0 "/Game/MyPlayer/Sounds/WeaponSouneds_Attenuation.WeaponSouneds_Attenuation" null null null)
      (set `self.Is Broken?` true)
      (`NiagaraFunctionLibrary.SpawnSystemAtLocation` "/Game/MyPlayer/MolotovBreak_NS.MolotovBreak_NS" (`SceneComponent.K2_GetComponentLocation` (`self.StaticMeshComponent`)))
      (bind _returnvalue_3 (`NiagaraFunctionLibrary.SpawnSystemAtLocation` "/Game/M5VFXVOL2/Niagara/Fire/NFire_Grd_02.NFire_Grd_02" (`.ImpactPoint` (`GameplayStatics.BreakHitResult` _outhit))))
      (`ActorComponent.K2_DestroyComponent` (`self.StaticMeshComponent`))
      (`GameplayStatics.PlaySoundAtLocation` "/Game/MyPlayer/Sounds/Sounds/cinematic-transition-flame-01.cinematic-transition-flame-01" (`self.K2_GetActorLocation`) (struct) 1.0 1.0 0.0 "/Game/MyPlayer/Sounds/WeaponSouneds_Attenuation.WeaponSouneds_Attenuation" null null null)
      (`|ExecutionSequence`
        (:`then_0`
          (bind _returnvalue_4 (`KismetSystemLibrary.K2_SetTimerDelegate` (delegate `CustomEvent`) 0.1 true))
          (`KismetSystemLibrary.Delay` 15.0)
          (`KismetSystemLibrary.K2_ClearAndInvalidateTimerHandle` _returnvalue_4))
        (:`then_1`
          (`KismetSystemLibrary.Delay` 15.0)
          (`ActorComponent.Deactivate` _returnvalue_3)
          (`KismetSystemLibrary.Delay` 1.0)
          (`self.K2_DestroyActor`))))))

(event `Throw`
  (params (Target :type "CameraComponent Object Reference"))
  (bind _staticmeshcomponent (`self.StaticMeshComponent`))
  (`PrimitiveComponent.SetSimulatePhysics` _staticmeshcomponent true)
  (`PrimitiveComponent.SetCollisionEnabled` (`self.StaticMeshComponent`) "QueryAndPhysics")
  (`PrimitiveComponent.AddImpulse` _staticmeshcomponent (+ (+ (* (`SceneComponent.GetForwardVector` Target) 3000.0) (* (`SceneComponent.GetUpVector` Target) 500.0)) (* (`SceneComponent.GetRightVector` Target) 50.0)) "None" false))

(fn `Hand Sway`
  (returns (SideMov :type "Float (double-precision)") (`Mouse X` :type "Float (double-precision)") (`Mouse Y` :type "Float (double-precision)"))
  (return 0.0 0.0 0.0))

(fn `Hand Sway 2`
  (returns (`Front Mov` :type "Float (double-precision)"))
  (return 0.0))

(fn `UserConstructionScript`)