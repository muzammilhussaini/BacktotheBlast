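; SmallAmmo_BP is a world pickup for 9mm bullets carrying an Amount of ammo.
; When Box1 is overlapped, it sends PickupAmmoMessage to the overlapping actor with the ammo type, itself and the amount, leaving the pickup logic to that actor.
; ShowInteractionWidget creates or removes a PickupSupply_UI prompt showing the item's name, image and amount.
; The Hand Sway functions only return zeros.
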(event `self.Show Interaction Widget`
  (params (Visibility :type Boolean))
  (if Visibility
    (bind _returnvalue (`|CreateWidget` "/Game/MyPlayer/Widget/PickupSupply_UI.PickupSupply_UI_C" null (`self.Amount`) "9.mm Bullets" "/Game/MyPlayer/Images/24482-8-ammunition-photos.24482-8-ammunition-photos"))
    (`UserWidget.AddToViewport` _returnvalue 0)
    (else
      (`/Engine/EditorBlueprintResources/StandardMacros.IsValid` _returnvalue
        (:`Is Valid`
          (`Widget.RemoveFromParent` _returnvalue))))))

(event `self.Box1.OnComponentBeginOverlap`
  (params (OverlappedComponent :type "PrimitiveComponent Object Reference") (OtherActor :type "Actor Object Reference") (OtherComp :type "PrimitiveComponent Object Reference") (OtherBodyIndex :type Integer) (bFromSweep :type Boolean) (SweepResult :type "HitResult Structure (by ref)"))
  (message `/Game/MyPlayer/OtherBlueprints/Player_BPI.Pickup Ammo` OtherActor "NewEnumerator0" self (`self.Amount`)))

(fn `Hand Sway`
  (returns (SideMov :type "Float (double-precision)") (`Mouse X` :type "Float (double-precision)") (`Mouse Y` :type "Float (double-precision)"))
  (return 0.0 0.0 0.0))

(fn `Hand Sway 2`
  (returns (`Front Mov` :type "Float (double-precision)"))
  (return 0.0))

(fn `UserConstructionScript`)