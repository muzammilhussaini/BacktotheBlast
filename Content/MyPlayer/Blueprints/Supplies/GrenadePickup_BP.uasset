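; Grenade pickup Blueprint that the player can interact with to collect one grenade.
; On BeginPlay it fills two widget components: an interact prompt and a supply card with name, icon and amount.
; An event toggles both widgets' visibility, and Interact passes the supply type, itself and the amount to the player through PickupSupplyMessage.
; The Hand Sway functions are stubs returning zero.
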(event `self.ReceiveBeginPlay`
  (bind _asinteract_ui (cast `/Game/MyPlayer/Widget/Interact_UI` (`WidgetComponent.GetUserWidgetObject` (`self.Widget`))))
  (set `/Game/MyPlayer/Widget/Interact_UI.Interact Text` "To Pickup" _asinteract_ui)
  (bind _aspickup_supply_ui (cast `/Game/MyPlayer/Widget/PickupSupply_UI` (`WidgetComponent.GetUserWidgetObject` (`self.Widget1`))))
  (set `/Game/MyPlayer/Widget/PickupSupply_UI.Name` "Grenade" _aspickup_supply_ui)
  (set `/Game/MyPlayer/Widget/PickupSupply_UI.Image` "/Game/MyPlayer/Images/Pi7_grenade.Pi7_grenade" _aspickup_supply_ui)
  (set `/Game/MyPlayer/Widget/PickupSupply_UI.Amount` 1 _aspickup_supply_ui))

(event `self.Show Interaction Widget`
  (params (Visibility :type Boolean))
  (`SceneComponent.SetVisibility` (`self.Widget`) Visibility false)
  (`SceneComponent.SetVisibility` (`self.Widget1`) Visibility false))

(event `self.Interact`
  (params (Player :type "Pawn Object Reference"))
  (message `/Game/MyPlayer/OtherBlueprints/Player_BPI.Pickup Supply` Player "NewEnumerator3" self 1))

(fn `Hand Sway`
  (returns (SideMov :type "Float (double-precision)") (`Mouse X` :type "Float (double-precision)") (`Mouse Y` :type "Float (double-precision)"))
  (return 0.0 0.0 0.0))

(fn `Hand Sway 2`
  (returns (`Front Mov` :type "Float (double-precision)"))
  (return 0.0))

(fn `UserConstructionScript`)