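; 2xScope is a weapon scope Blueprint with a SceneCaptureComponent2D that renders to a render target while on the player's current weapon.
; It caches Player_BP on BeginPlay, then checks every Tick whether it is the ScopeObject of the current or other weapon.
; The current weapon's scope captures into 8xScope_RenderTarget, despite the 2x name, while the other weapon's scope has its texture target cleared.
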(event `self.ReceiveBeginPlay`
  (bind _asplayer_bp (cast `/Game/MyPlayer/Player_BP` (`GameplayStatics.GetPlayerCharacter` 0)))
  (set `self.As Player BP` _asplayer_bp))

(event `self.ReceiveTick`
  (params (DeltaSeconds :type "Float (single-precision)"))
  (bind _other_weapon_object (`/Game/MyPlayer/Player_BP.Other Weapon Object` (`self.As Player BP`)))
  (bind _current_weapon_object (`/Game/MyPlayer/Player_BP.Current Weapon Object` (`self.As Player BP`)))
  (`|ExecutionSequence`
    (:`then_0`
      (`/Engine/EditorBlueprintResources/StandardMacros.IsValid` _current_weapon_object
        (:`Is Valid`
          (if (== (`/Game/MyPlayer/Blueprints/WeaponswitChilds/WeaponBase_BP.Scope Object` _current_weapon_object) self)
            (set `SceneCaptureComponent2D.TextureTarget` "/Game/MyPlayer/8xScope_RenderTarget.8xScope_RenderTarget" (`self.SceneCaptureComponent2D`))))))
    (:`then_1`
      (`/Engine/EditorBlueprintResources/StandardMacros.IsValid` _other_weapon_object
        (:`Is Valid`
          (if (== (`/Game/MyPlayer/Blueprints/WeaponswitChilds/WeaponBase_BP.Scope Object` _other_weapon_object) self)
            (set `SceneCaptureComponent2D.TextureTarget` null (`self.SceneCaptureComponent2D`))))))))

(fn `UserConstructionScript`)